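; Placeholder enemy spawner actor that endlessly spawns a configurable enemy class at its own transform, starting shortly after BeginPlay.
; Each spawn ignores collision, then teleports the new actor up by its bounds' half-height so it rests above the spawn point.
; PerformSpawn then re-arms a timer to itself, randomizing the interval around MinDelayBetweenSpawns through a positive or negative initial start delay.
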(event `SetSpawnTimer`
  (`KismetSystemLibrary.K2_SetTimerDelegate` (delegate `PerformSpawn`) (`self.MinDelayBetweenSpawns`) false (`KismetMathLibrary.RandomFloatInRange` (* (`self.MinDelayBetweenSpawns`) -1.0) (`self.MinDelayBetweenSpawns`))))

(event `self.ReceiveBeginPlay`
  (`KismetSystemLibrary.Delay` 2.0)
  (`self.PerformSpawn`))

(event `PerformSpawn`
  (bind (_returnvalue_location _returnvalue_rotation) (`KismetMathLibrary.BreakTransform` (`self.GetTransform`)))
  (bind _returnvalue (`|SpawnActorFromClass` (`self.EnemyToSpawnClass`) (`KismetMathLibrary.MakeTransform` _returnvalue_location _returnvalue_rotation) "AlwaysSpawn" "OverrideRootScale" self null))
  (`self.K2_AddActorWorldOffset` _returnvalue (`KismetMathLibrary.MakeVector` 0.0 0.0 (.z (`.BoxExtent` (`self.GetActorBounds` _returnvalue false false)))) false true)
  (`self.SetSpawnTimer`))

(fn `UserConstructionScript`)