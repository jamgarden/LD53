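; Main game mode for a cart escort game, handling cart spawning, win/lose conditions and letter screens.
; On BeginPlay it spawns BP_Cart between tagged TargetPoints, starts it and shows an intro letter widget.
; Reaching the destination wins, while escort-too-far or enemy-touch events lose once their counters exceed thresholds.
; EndGame fires only once, showing the result letter; Tick prints both counters for debugging.
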(event `EndGame`
  (params (WonGame :type Boolean))
  ;[1 1 1] End Game
  (if (not (`self.GameEnded`))
    (set `self.GameEnded` true)
    (`self.CreateLetterWidget` (select `bool` WonGame :`false` "NewEnumerator1" :`true` "NewEnumerator0" :!type "/Game/FirstPerson/Blueprints/LetterMode Enum"))))

(event `TriggerLose`
  ;[1 1 1] Fail / Succeed
  (`self.EndGame` false))

(event `TriggerWin`
  ;[1 1 1] Fail / Succeed
  (`self.EndGame` true))

(event `CreateLetterWidget`
  (params (LetterMode :type "/Game/FirstPerson/Blueprints/LetterMode Enum" :default "NewEnumerator0"))
  ;[1 1 1] Create Letter Widget
  (bind _returnvalue (`|CreateWidget` "/Game/FirstPerson/Blueprints/LetterWidget.LetterWidget_C"))
  (set `/Game/FirstPerson/Blueprints/LetterWidget.LetterMode` LetterMode _returnvalue)
  (`UserWidget.AddToViewport` _returnvalue 0))

(event `self.ReceiveBeginPlay`
  (`parent.ReceiveBeginPlay`)
  (`self.RestartCart`)
  (`self.CreateLetterWidget` "NewEnumerator2"))

(event `RestartCart`
  (bind _cart (`self.Cart`))
  (`|ExecutionSequence`
    (:`then_0`
      (bind _targetpoint (`self.GetTargetPointWithTag` "cart")
        (:`Found`
          (set `self.CartSpawnPoint` _targetpoint))
        (:`Not Found`
          (`self.RestartPlayer` (`GameplayStatics.GetPlayerController` 0)))))
    (:`then_1`
      (bind _targetpoint_2 (`self.GetTargetPointWithTag` "cartdestination")
        (:`Found`
          (set `self.CartDestinationPoint` _targetpoint_2))
        (:`Not Found`
          (`self.RestartPlayer` (`GameplayStatics.GetPlayerController` 0)))))
    (:`then_4`
      (bind _cart_2 (`self.Cart`)
        (:`then`
          (`self.K2_DestroyActor` _cart_2))
        (:`else`
          _))
      (bind _returnvalue (`|SpawnActorFromClass` "/Game/Blueprints/NPCs/BP_Cart.BP_Cart_C" (`self.GetTransform` (`self.CartSpawnPoint`)) "AlwaysSpawn" "OverrideRootScale" self (`self.CartDestinationPoint`) null))
      (set `self.Cart` _returnvalue)
      (`|ExecutionSequence`
        (:`then_0`
          ;[1 1 1] WIN CONDITIONS
          (add `/Game/Blueprints/NPCs/BP_Cart.OnDestinationReached` _cart (delegate `HandleOnDestinationReached`)))
        (:`then_1`
          ;[1 1 1] LOSE CONDITIONS
          (add `/Game/Blueprints/NPCs/BP_Cart.OnEscortTooFar` _cart (delegate `HandleOnEscortTooFar`)))
        (:`then_2`
          (add `/Game/Blueprints/NPCs/BP_Cart.OnEnemyTouched` _cart (delegate `HandleOnEnemyTouched`)))
        (:`then_3`
          (`/Game/Blueprints/NPCs/BP_Cart.Start` (`self.Cart`)))))))

(event `HandleOnDestinationReached`
  ;[1 1 1] WIN CONDITIONS
  (`self.TriggerWin`))

(event `self.K2_OnRestartPlayer`
  (params (NewPlayer :type "Controller Object Reference"))
  (set `self.CurrentPlayerPawn` (`Controller.K2_GetPawn` NewPlayer)))

(event `HandleOnEscortTooFar`
  ;[1 1 1] LOSE CONDITIONS
  (`/Engine/EditorBlueprintResources/StandardMacros.IncrementInt` (`self.EscortExceededDistanceCtr`)
    (:`  `
      (if (> (`self.EscortExceededDistanceCtr`) (`self.EscortExceededDistanceThreshold`))
        (`self.TriggerLose`)))))

(event `self.ReceiveTick`
  (params (DeltaSeconds :type "Float (single-precision)"))
  (`KismetSystemLibrary.PrintString` (`KismetTextLibrary.Conv_TextToString` (`|FormatText` "Exceeded Distance: {dist} \nTouched: {touch}" (`self.EscortExceededDistanceCtr`) (`self.EnemyTouchedCtr`))) true false (struct :`G` 0.66 :`B` 1.0 :`A` 1.0) (* DeltaSeconds 1.0)))

(event `HandleOnEnemyTouched`
  ;[1 1 1] LOSE CONDITIONS
  (`/Engine/EditorBlueprintResources/StandardMacros.IncrementInt` (`self.EnemyTouchedCtr`)
    (:`  `
      (if (> (`self.EnemyTouchedCtr`) (`self.EnemyTouchedThreshold`))
        (`self.TriggerLose`)))))

(fn `UserConstructionScript`)