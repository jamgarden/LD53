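; Enemy character Blueprint that displays its health in a widget and ragdolls on death.
; On BeginPlay it caches the placeholder health widget, which the attributes component's health-change event then updates, also playing an attack sound cue.
; On death it disables capsule collision, enables mesh physics and sets a short lifespan.
; A separate any-damage sound handler exists, but its binding never runs.
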(event `self.ReceiveBeginPlay`
  (`parent.ReceiveBeginPlay`)
  (bind _aswbp_enemy_character_placeholder (cast `/Game/Blueprints/UI/WBP_EnemyCharacter_Placeholder` (`WidgetComponent.GetWidget` (`self.Widget_Health_Placeholder`)))
    (:`then`
      (bind _output_get (set `self.HealthWidget` _aswbp_enemy_character_placeholder))
      (`/Game/Blueprints/UI/WBP_EnemyCharacter_Placeholder.SetHealthPercentage` _output_get (`/Game/Blueprints/NPCs/BP_AttributesComponent.GetHealthPercent` (`self.BP_AttributesComponent`))))
    (:`CastFailed`
      (`KismetSystemLibrary.LogString` "Invalid cast to widget enemy character."))))

(event `self.BP_AttributesComponent.OnHealthChanged`
  (params (HealthDelta :type "Float (double-precision)"))
  (if (> (`KismetMathLibrary.Abs` HealthDelta) 0.0)
    (bind _healthwidget (`self.HealthWidget`)
      (:`then`
        (`/Game/Blueprints/UI/WBP_EnemyCharacter_Placeholder.SetHealthPercentage` _healthwidget (`/Game/Blueprints/NPCs/BP_AttributesComponent.GetHealthPercent` (`self.BP_AttributesComponent`)))
        (`GameplayStatics.PlaySoundAtLocation` "/Game/Audio/SFX/OsteomechanicumAttack2_Cue.OsteomechanicumAttack2_Cue" (0.0 0.0 0.0) (struct) 2.0 1.0 0.0 "/Game/FirstPerson/Blueprints/MyAttenuation.MyAttenuation" null null null))
      (:`else`))))

(event `self.BP_AttributesComponent.OnDeath`
  (`PrimitiveComponent.SetCollisionEnabled` (`self.CapsuleComponent`) "NoCollision")
  (`PrimitiveComponent.SetCollisionProfileName` (`self.Mesh`) "PhysicsActor" true)
  (`PrimitiveComponent.SetSimulatePhysics` (`self.Mesh`) true)
  (`self.SetLifeSpan` 5.0))

(event `OnTakeAnyDamage_Event` :!signature `self.OnTakeAnyDamage`
  (params (DamagedActor :type "Actor Object Reference") (Damage :type "Float (single-precision)") (DamageType :type "DamageType Object Reference") (InstigatedBy :type "Controller Object Reference") (DamageCauser :type "Actor Object Reference"))
  (`GameplayStatics.PlaySoundAtLocation` "/Game/Audio/SFX/OsteomechanicumAttack2.OsteomechanicumAttack2" (`self.GetNavAgentLocation`) (struct) 1.0 1.0 0.0 "/Game/FirstPerson/Blueprints/MyAttenuation.MyAttenuation" null null null))

(fn `UserConstructionScript`
  (`parent.UserConstructionScript`))