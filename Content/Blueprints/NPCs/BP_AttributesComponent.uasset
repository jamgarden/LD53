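; Attributes component in the NPCs folder that tracks health, starting from a clamped initial value, and reports changes and death.
; ApplyToHealth is the central function: it adds an amount, clamps to zero and max, fires OnDeath once at zero, then OnHealthChanged with the actual delta.
; TakeDamage routes damage through ApplyToHealth, and GetHealthPercent returns health over max using a safe divide.
; Tick is unused.
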(event `self.ReceiveBeginPlay`
  (set `self.Health` (`KismetMathLibrary.FClamp` (`self.InitialHealth`) 0.0 (`self.MaxHealth`))))

(fn `ApplyToHealth`
  (params (HealthAmount :type "Float (double-precision)"))
  (locals (LocalHealthDelta :type "Float (double-precision)") (LocalOldHealth :type "Float (double-precision)" :default 0.0))
  (set `local.LocalOldHealth` (`self.Health`))
  (bind _output_get (set `self.Health` (`KismetMathLibrary.FClamp` (+ HealthAmount (`self.Health`)) 0.0 (`self.MaxHealth`))))
  (`|ExecutionSequence`
    (:`then_0`
      (if (<= _output_get 0.0)
        (`/Engine/EditorBlueprintResources/StandardMacros.DoOnce` false
          (:`Completed`
            (`self.OnDeath`)))))
    (:`then_1`
      (bind _output_get_2 (set `local.LocalHealthDelta` (- (`self.Health`) (`local.LocalOldHealth`))))
      (`self.OnHealthChanged` _output_get_2))))

(fn `GetHealthPercent`
  (returns (HealthPercent :type "Float (double-precision)"))
  (return (`KismetMathLibrary.SafeDivide` (`self.Health`) (`self.MaxHealth`))))

(fn `TakeDamage`
  (params (DamageAmount :type "Float (double-precision)"))
  (bind _result (`/Engine/EditorBlueprintResources/StandardMacros.NegateFloat` DamageAmount)
    (:`  `
      (`self.ApplyToHealth` _result))))