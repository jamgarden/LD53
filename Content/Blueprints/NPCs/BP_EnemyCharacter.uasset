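; Enemy NPC character Blueprint with a health display and a ragdoll death.
; On BeginPlay it caches the health placeholder widget and sets its initial percentage from the attributes component.
; Health changes refresh the widget and play a 2D sound.
; Death disables capsule collision, turns the mesh into a physics ragdoll, plays an attenuated death sound at the hit location and sets a short lifespan before removal.
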(event `self.ReceiveBeginPlay`
  (`parent.ReceiveBeginPlay`)
  (bind _aswbp_enemy_character_placeholder (cast `/Game/Blueprints/UI/WBP_EnemyCharacter_Placeholder` (`WidgetComponent.GetWidget` (`self.Widget_Health_Placeholder`)))
    (:`then`
      (bind _output_get (set `self.HealthWidget` _aswbp_enemy_character_placeholder))
      (`/Game/Blueprints/UI/WBP_EnemyCharacter_Placeholder.SetHealthPercentage` _output_get (`/Game/Blueprints/NPCs/BP_AttributesComponent.GetHealthPercent` (`self.BP_AttributesComponent`))))
    (:`CastFailed`
      (`KismetSystemLibrary.LogString` "Invalid cast to widget enemy character."))))

(event `self.BP_AttributesComponent.OnHealthChanged`
  (params (HealthDelta :type "Float (double-precision)") (HitResult :type "HitResult Structure"))
  (if (> (`KismetMathLibrary.Abs` HealthDelta) 0.0)
    (bind _healthwidget (`self.HealthWidget`)
      (:`then`
        (`/Game/Blueprints/UI/WBP_EnemyCharacter_Placeholder.SetHealthPercentage` _healthwidget (`/Game/Blueprints/NPCs/BP_AttributesComponent.GetHealthPercent` (`self.BP_AttributesComponent`)))
        (`GameplayStatics.PlaySound2D` "/Game/Audio/SFX/OsteomechanicumAttack2_Cue.OsteomechanicumAttack2_Cue" 1.0 1.0 0.0 null null))
      (:`else`))))

(event `self.BP_AttributesComponent.OnDeath`
  (params (HitResult :type "HitResult Structure"))
  (`PrimitiveComponent.SetCollisionEnabled` (`self.CapsuleComponent`) "NoCollision")
  (`PrimitiveComponent.SetCollisionProfileName` (`self.Mesh`) "PhysicsActor" true)
  (`PrimitiveComponent.SetSimulatePhysics` (`self.Mesh`) true)
  (`GameplayStatics.PlaySoundAtLocation` "/Game/Audio/SFX/MonsterDeath.MonsterDeath" (`.Location` (`GameplayStatics.BreakHitResult` HitResult)) (struct) 3.0 1.0 0.0 "/Game/FirstPerson/Blueprints/MyAttenuation.MyAttenuation" null null null)
  (`self.SetLifeSpan` 5.0))

(event `self.OnLaunched`
  (params (LaunchVelocity :type "Vector Structure") (bXYOverride :type Boolean) (bZOverride :type Boolean)))

(event `self.OnLanded`
  (params (Hit :type "HitResult Structure (by ref)")))

(fn `UserConstructionScript`
  (`parent.UserConstructionScript`))