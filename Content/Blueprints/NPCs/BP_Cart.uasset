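; BP_Cart is an escort-mission cart pawn that drives to a destination actor via AIMoveTo once Start is called.
; An overlap sphere sized by EscortRadius tracks the player as Escort, while a delayed Tick check fires OnEscortTooFar on a cooldown when none is present.
; Enemies hitting the cube are launched away at a random pitch, and dispatchers report touches and arrival.
; HasEscortExceededMaxDistance is defined but unused here.
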(event `self.PlayerEscortOverlapSphere.OnComponentBeginOverlap`
  (params (OverlappedComponent :type "PrimitiveComponent Object Reference") (OtherActor :type "Actor Object Reference") (OtherComp :type "PrimitiveComponent Object Reference") (OtherBodyIndex :type Integer) (bFromSweep :type Boolean) (SweepResult :type "HitResult Structure (by ref)"))
  (bind _asbp_first_person_character (cast `/Game/FirstPerson/Blueprints/BP_FirstPersonCharacter` OtherActor))
  (set `self.Escort` _asbp_first_person_character))

(event `self.PlayerEscortOverlapSphere.OnComponentEndOverlap`
  (params (OverlappedComponent :type "PrimitiveComponent Object Reference") (OtherActor :type "Actor Object Reference") (OtherComp :type "PrimitiveComponent Object Reference") (OtherBodyIndex :type Integer))
  (if (`GameplayStatics.ObjectIsA` OtherActor "/Game/FirstPerson/Blueprints/BP_FirstPersonCharacter.BP_FirstPersonCharacter_C")
    (set `self.Escort` null)))

(event `self.ReceiveTick`
  (params (DeltaSeconds :type "Float (single-precision)"))
  (`|ExecutionSequence`
    (:`then_0`
      (`KismetSystemLibrary.Delay` (`self.EscortCheckDelay`))
      (goto _label :!via `Open`))
    (:`then_1`
      (`/Engine/EditorBlueprintResources/StandardMacros.Gate` true :!label _label
        (:`Exit`
          (`KismetSystemLibrary.PrintString` "Checking Escort Distance" true false (struct :`G` 0.66 :`B` 1.0 :`A` 1.0) (`GameplayStatics.GetWorldDeltaSeconds`))
          (`KismetSystemLibrary.Delay` (`self.EscortIntervalCheck`))
          (`self.Escort`
            (:`then`)
            (:`else`
              (`KismetSystemLibrary.Delay` 1.0)
              (`KismetSystemLibrary.LogString` "Warning: No escort.")
              (`/Engine/EditorBlueprintResources/StandardMacros.DoOnce` false :!label _label_2
                (:`Completed`
                  (`self.OnEscortTooFar`)
                  (`KismetSystemLibrary.Delay` (`self.EscortReportCooldown`))
                  (goto _label_2 :!via `Reset`))))))))))

(event `self.ReceivePossessed`
  (params (NewController :type "Controller Object Reference"))
  (bind _asbp_cart_controller (cast `/Game/Blueprints/NPCs/BP_CartController` NewController))
  (set `self.CartController` _asbp_cart_controller))

(event `self.Cube.OnComponentHit`
  (params (HitComponent :type "PrimitiveComponent Object Reference") (OtherActor :type "Actor Object Reference") (OtherComp :type "PrimitiveComponent Object Reference") (NormalImpulse :type "Vector Structure") (Hit :type "HitResult Structure (by ref)"))
  (bind _asbp_enemy_character_base (cast `/Game/Blueprints/NPCs/BP_EnemyCharacter_Base` OtherActor))
  (`|ExecutionSequence`
    (:`then_0`
      (`/Engine/EditorBlueprintResources/StandardMacros.IsValid` _asbp_enemy_character_base
        (:`Is Valid`
          (`self.LaunchCharacter` _asbp_enemy_character_base (* (`KismetMathLibrary.Normal` (`KismetMathLibrary.GreaterGreater_VectorRotator` (- (`self.K2_GetActorLocation` _asbp_enemy_character_base) (`self.K2_GetActorLocation`)) (`KismetMathLibrary.MakeRotator` 0.0 (`KismetMathLibrary.RandomFloatInRange` 45.0 80.0)))) (`self.LaunchVelocity`)) true true))))
    (:`then_1`
      (`self.OnEnemyTouched`))))

(event `Start`
  (`self.CartController`
    (:`then`
      (bind _destinationactor (`self.DestinationActor`)
        (:`then`
          (`|AIMoveTo` self (0.0 0.0 0.0) _destinationactor 20.0 true
            (:`OnSuccess`
              (`self.OnDestinationReached`))
            (:`OnFail`
              (`KismetSystemLibrary.PrintString` "Error: Failed to move to cart destination."))))
        (:`else`
          (`KismetSystemLibrary.PrintString` "Error: Invalid destination actor."))))
    (:`else`
      (`KismetSystemLibrary.LogString` "Error: Invalid cart controller."))))

(fn `HasEscortExceededMaxDistance`
  (returns (ReturnValue :type Boolean))
  (bind _escort (`self.Escort`)
    (:`then`
      (return (> (`KismetMathLibrary.VSize` (- (`self.K2_GetActorLocation` _escort) (`self.K2_GetActorLocation`))) (`self.MaxDistance`))))
    (:`else`)))

(fn `UserConstructionScript`
  (`SphereComponent.SetSphereRadius` (`self.PlayerEscortOverlapSphere`) (`self.EscortRadius`) true))